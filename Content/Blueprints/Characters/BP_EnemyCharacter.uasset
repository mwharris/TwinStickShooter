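; Enemy character for the twin-stick game that damages the hero on contact and awards score when killed.
; Overlapping the hero starts a looping DamageHero timer paced by attacks per second, cleared when the overlap ends.
; Lethal damage ignores pawn and world-dynamic collision, detaches the controller, increments score, then after a delay notifies the GameMode and destroys the actor.
; The construction script tints the mesh through a dynamic material using the enemy color.
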(event Custom|DamageHero
  ;[1 1 1] Deal damage to the hero everytime DamageHero is called
  (Default|AffectHealth (Variables|Default|GetHeroCharacter) (Variables|Default|GetDamage)))

(event EventAffectHealth
  (params (Delta :type Float%20%28single-precision%29))
  (bind _gamemoderef (Variables|Default|GetGameModeRef))
  (bind _capsulecomponent (Variables|Default|GetCapsuleComponent))
  ;[1 1 1] Taking damage
  (Class|BaseCharacter|CalculateHealth Delta)
  ;[1 1 1] Check for dead
  (if (Variables|Default|GetIsDead)
    ;[1 1 1] Deactivate collisions and input
    (Collision|SetCollisionResponsetoChannel _capsulecomponent "ECC_WorldDynamic" "ECR_Ignore")
    (Collision|SetCollisionResponsetoChannel _capsulecomponent "ECC_Pawn" "ECR_Ignore")
    (Class|Pawn|DetachfromControllerPendingDestroy)
    ;[1 1 1] Tell GameMode to increment score
    (Default|IncrementScore (Variables|Default|GetGameModeRef) (Variables|Default|GetEnemyScore))
    ;[1 1 1] Destroy the Actor after a delay
    (Utilities|FlowControl|Delay 3.0)
    (Utilities|IsValid _gamemoderef
      (:Is%20Valid
        (Default|EnemyDied _gamemoderef)
        (Actor|DestroyActor)))))

(event Collision|EventActorBeginOverlap
  (params (OtherActor :type Actor%20Object%20Reference))
  ;[1 1 1] Call DamageHero when our attack hitbox overlaps the player
  (if (== OtherActor (Variables|Default|GetHeroCharacter))
    (Utilities|Time|SetTimerbyEvent (delegate Custom|DamageHero) (/ 1.0 (Variables|Default|GetAttacksPerSecond)) true)))

(event EventBeginPlay
  ;[1 1 1] Cache a reference to the Hero Character
  (bind _asbp_hero_character (Utilities|Casting|CastToBP_HeroCharacter (Game|GetPlayerCharacter 0)))
  (Variables|Default|SetHeroCharacter _asbp_hero_character)
  ;[1 1 1] Get a reference to the GameMode
  (bind _asbp_twin_stick_game_mode (Utilities|Casting|CastToBP_TwinStickGameMode (Game|GetGameMode)))
  (Variables|Default|SetGameModeRef _asbp_twin_stick_game_mode))

(event Collision|EventActorEndOverlap
  (params (OtherActor :type Actor%20Object%20Reference))
  ;[1 1 1] Clear DamageHero timer when we're no longer overlapping
  (if (== OtherActor (Variables|Default|GetHeroCharacter))
    (Utilities|Time|ClearTimerbyFunctionName 0 "DamageHero")))

(fn ConstructionScript
  (bind _returnvalue (Rendering|Material|CreateDynamicMaterialInstance (Variables|Character|GetMesh) 0 0 "None" :!class /Script/Engine.PrimitiveComponent))
  (bind _output_get (Variables|Default|SetDynamicMaterial _returnvalue))
  (Rendering|Material|SetVectorParameterValue _output_get "BodyColor" (Variables|Default|GetEnemyColor) :!class /Script/Engine.MaterialInstanceDynamic))