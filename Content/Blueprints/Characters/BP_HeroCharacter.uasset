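; Player hero character for a twin-stick shooter, handling movement, aimed firing, health display and respawn.
; On BeginPlay it spawns a weapon on the GunSocket, records its spawn transform in the game mode and creates the HUD.
; Move axes drive world-space movement, while look axes past a deadzone set control rotation and hold the weapon trigger.
; Damage updates the HUD, and death disables input, then after a delay requests respawn and destroys weapon and character.
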(event EventBeginPlay
  (bind _mesh (Variables|Character|GetMesh))
  (Utilities|FlowControl|Sequence
    (:then_0
      (bind _returnvalue (Game|SpawnActorfromClass "/Game/Blueprints/Actors/BP_Weapon.BP_Weapon_C" (Transformation|GetWorldTransform _mesh) "Undefined" 0 0))
      (bind _output_get (Variables|Default|SetWeapon _returnvalue))
      (Transformation|AttachComponentToComponent _output_get _mesh "GunSocket" "SnapToTarget" "SnapToTarget" "KeepWorld" true))
    (:then_1
      (bind _asbp_twin_stick_game_mode (Utilities|Casting|CastToBP_TwinStickGameMode (Game|GetGameMode)))
      (bind _output_get_2 (Variables|Default|SetGameModeRef _asbp_twin_stick_game_mode))
      (Variables|/Game/Blueprints/GameModes/BP_TwinStickGameMode.BP_TwinStickGameMode_C|SetPlayerSpawnTransform _output_get_2 (Transformation|GetActorTransform)))
    (:then_2
      (bind _returnvalue_2 (UserInterface|CreateWidget "/Game/UI/WBP_HUD.WBP_HUD_C"))
      (bind _output_get_3 (Variables|Default|SetHUDRef _returnvalue_2))
      (UserInterface|Viewport|AddtoViewport _output_get_3 0))))

(event EventAffectHealth
  (params (Delta :type Float%20%28single-precision%29))
  ;[1 1 1] Taking Damage
  (bind _returnvalue (Class|BaseCharacter|CalculateHealth Delta))
  (Default|UpdateHealth (Variables|Default|GetHUDRef) _returnvalue)
  ;[1 1 1] Handling death + respawning
  (if (Variables|Default|GetIsDead)
    (Input|DisableInput (Game|GetPlayerController 0))
    (Utilities|FlowControl|Delay 3.0)
    (Default|RespawnPlayer (Variables|Default|GetGameModeRef))
    (Actor|DestroyActor (Variables|Default|GetWeapon))))

(event Input|AxisEvents|InputAxisMoveUp
  (params (AxisValue :type Float%20%28single-precision%29))
  ;[1 1 1] Movement input handling
  (Pawn|Input|AddMovementInput "1.000000, 0, 0" AxisValue false))

(event Input|AxisEvents|InputAxisMoveRight
  (params (AxisValue :type Float%20%28single-precision%29))
  ;[1 1 1] Movement input handling
  (Pawn|Input|AddMovementInput "0,1.000000, 0" AxisValue false))

(event Input|AxisEvents|InputAxisLookUp
  (params (AxisValue :type Float%20%28single-precision%29))
  (bind _weapon (Variables|Default|GetWeapon))
  ;[1 1 1] Look input handling + firing weapon
  (if (> (Math|Vector|VectorLength (Math|Vector|MakeVector AxisValue (stale Input|AxisEvents|InputAxisLookRight AxisValue) 0.0)) 0.25)
    (Pawn|SetControlRotation (Pawn|GetController) (Math|Conversions|RotationFromXVector (Math|Vector|MakeVector AxisValue (stale Input|AxisEvents|InputAxisLookRight AxisValue) 0.0)))
    (Default|PullTrigger _weapon)
    (else
      (Default|ReleaseTrigger _weapon))))

(event Input|AxisEvents|InputAxisLookRight
  (params (AxisValue :type Float%20%28single-precision%29))
  (bind _weapon (Variables|Default|GetWeapon))
  ;[1 1 1] Look input handling + firing weapon
  (if (> (Math|Vector|VectorLength (Math|Vector|MakeVector (stale Input|AxisEvents|InputAxisLookUp AxisValue) AxisValue 0.0)) 0.25)
    (Pawn|SetControlRotation (Pawn|GetController) (Math|Conversions|RotationFromXVector (Math|Vector|MakeVector (stale Input|AxisEvents|InputAxisLookUp AxisValue) AxisValue 0.0)))
    (Default|PullTrigger _weapon)
    (else
      (Default|ReleaseTrigger _weapon))))

(fn ConstructionScript)