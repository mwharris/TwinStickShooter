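; BP_Weapon is an automatic weapon actor that spawns BP_Projectile actors while its trigger is held.
; PullTrigger passes through a DoOnce, fires immediately, then starts a looping timer on Fire with an interval derived from RoundsPerSecond.
; Fire spawns each projectile at the ProjectileSpawnPoint world transform.
; ReleaseTrigger clears the timer and resets the DoOnce, so the next pull fires at once with no fire-rate cooldown between pulls.
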(event Custom|Fire
  ;[1 1 1] Actually fire the weapon: spawn BP_Projectiles
  (Game|SpawnActorfromClass "/Game/Blueprints/Actors/BP_Projectile.BP_Projectile_C" (Transformation|GetWorldTransform (Variables|Default|GetProjectileSpawnPoint)) "Undefined" 0 0))

(event Custom|PullTrigger
  ;[1 1 1] Create a timer that will repeatedly call the Fire event ever 1/X seconds
  (Utilities|FlowControl|DoOnce false
    (:Completed
      (CallFunction|Fire)
      (Utilities|Time|SetTimerbyFunctionName 0 "Fire" (/ 1.0 (Variables|Default|GetRoundsPerSecond)) true))))

(event Custom|ReleaseTrigger
  ;[1 1 1] Clear the timer set by PullTrigger and Reset the DoOnce
  (Utilities|Time|ClearTimerbyFunctionName 0 "Fire")
  ;[1 1 1] Create a timer that will repeatedly call the Fire event ever 1/X seconds
  (Utilities|FlowControl|DoOnce false) ; enters at Reset
)

(fn ConstructionScript)