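; BP_EnemySpawner is an actor that spawns BP_EnemyCharacter AI in the twin-stick game.
; It caches BP_TwinStickGameMode on BeginPlay.
; Its SpawnEnemy event, not triggered within this Blueprint, checks the game mode's spawned count against MaxEnemies, then spawns an enemy at a random point in SpawnVolume.
; It then notifies the game mode through EnemySpawned, validating the reference only at that step.
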(event Custom|SpawnEnemy
  (bind _spawn_volume (Variables|Default|GetSpawn%20Volume))
  (bind _gamemoderef (Variables|Default|GetGameModeRef))
  (if (< (Variables|/Game/Blueprints/GameModes/BP_TwinStickGameMode.BP_TwinStickGameMode_C|GetNumSpawnedEnemies (Variables|Default|GetGameModeRef)) (Variables|Default|GetMaxEnemies))
    (AI|SpawnAIFromClass "/Game/Blueprints/Characters/BP_EnemyCharacter.BP_EnemyCharacter_C" 0 (Math|Random|RandomPointinBoundingBox (Transformation|GetWorldLocation _spawn_volume) (Components|Box|GetScaledBoxExtent _spawn_volume)) "0, 0, 0" false 0)
    (Utilities|IsValid _gamemoderef
      (:Is%20Valid
        (Default|EnemySpawned _gamemoderef)))))

(event EventBeginPlay
  (bind _asbp_twin_stick_game_mode (Utilities|Casting|CastToBP_TwinStickGameMode (Game|GetGameMode)))
  (Variables|Default|SetGameModeRef _asbp_twin_stick_game_mode))

(fn ConstructionScript)